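; First-person player character that spawns a BP_Rifle on its hand socket and handles Enhanced Input movement, look, jump, sprint, crouch and aim.
; Crouch toggles through a FlipFlop, with a timeline resizing the capsule.
; Sprint raises walk speed and animates camera FOV, while crouching, jumping or aiming mid-run cancels it through a shared Stop event.
; A short camera line trace each tick sets CloseToWall for procedural gun handling.
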(event `self.ReceiveBeginPlay`
  ;[0.01938 0.01938 0.01938] Adding the controll Mappings
  (`EnhancedInputSubsystemInterface.AddMappingContext` (pcsubsystem `EnhancedInputLocalPlayerSubsystem` (`GameplayStatics.GetPlayerController` 0)) "/Game/Hunters_Field/Data/IMC_GameInput.IMC_GameInput" 0 (struct))
  ;[0.01938 0.01938 0.01938] Spawning the rifle on play
  (bind _returnvalue (`|SpawnActorFromClass` "/Game/Hunters_Field/Core/BP_Rifle.BP_Rifle_C" (`KismetMathLibrary.MakeTransform` (0.0 0.0 0.0)) "Undefined" "MultiplyWithRoot" null null))
  (`self.K2_AttachToComponent` _returnvalue (`self.Mesh`) "ik_hand_gun" "SnapToTarget" "SnapToTarget" "SnapToTarget" true))

(event `Custom Crouch`
  ;[0.0137 0.0137 0.0137] Crouch
  ;;[0.0185 0.0185 0.0185] Creating the Crouch Event
  (set `self.bCrouched?` true)
  (`self.Stop`)
  (set `CharacterMovementComponent.MaxWalkSpeed` 350.0 (`self.CharacterMovement`))
  (bind (_direction _crouch_time) (`Timeline|Crouch Timeline` :!label _label)
    (:`Update`
      (`CapsuleComponent.SetCapsuleHalfHeight` (`self.CapsuleComponent`) _crouch_time true))))

(event `EnhancedInput|/Game/Hunters_Field/Data/IA_Movements`
  (params (ActionValue :type "Vector2D Structure") (ElapsedSeconds :type "Float (double-precision)") (TriggeredSeconds :type "Float (double-precision)") (InputAction :type "InputAction Object Reference" :default "/Game/Hunters_Field/Data/IA_Movements.IA_Movements"))
  ;[0.01938 0.01938 0.01938] Movement Inputs
  (:`Triggered`
    (`self.AddMovementInput` (* (`self.GetActorRightVector`) ActionValue_X))
    (`self.AddMovementInput` (* (`self.GetActorForwardVector`) ActionValue_Y))))

(event `Custom UnCrouch`
  ;[0.0137 0.0137 0.0137] Crouch
  ;;[0.0185 0.0185 0.0185] Creating the Crouch Event
  (set `self.bCrouched?` false)
  (set `CharacterMovementComponent.MaxWalkSpeed` 500.0 (`self.CharacterMovement`))
  (goto _label :!via `Reverse`))

(event `EnhancedInput|/Game/Hunters_Field/Data/IA_Camera`
  (params (ActionValue :type "Vector2D Structure") (ElapsedSeconds :type "Float (double-precision)") (TriggeredSeconds :type "Float (double-precision)") (InputAction :type "InputAction Object Reference" :default "/Game/Hunters_Field/Data/IA_Camera.IA_Camera"))
  ;[0.01938 0.01938 0.01938] Mouse Controles
  (:`Triggered`
    (`self.AddControllerYawInput` ActionValue_X)
    (`self.AddControllerPitchInput` (* ActionValue_Y -1.0))))

(event `EnhancedInput|/Game/Hunters_Field/Data/IA_Crouch`
  (params (ActionValue :type Boolean) (ElapsedSeconds :type "Float (double-precision)") (TriggeredSeconds :type "Float (double-precision)") (InputAction :type "InputAction Object Reference" :default "/Game/Hunters_Field/Data/IA_Crouch.IA_Crouch"))
  ;[0.0137 0.0137 0.0137] Crouch
  ;;[0.01938 0.01938 0.01938] Crouch calling
  (:`Triggered`
    (`/Engine/EditorBlueprintResources/StandardMacros.DoOnce` false :!label _label_2
      (:`Completed`
        (`/Engine/EditorBlueprintResources/StandardMacros.FlipFlop`
          (:`A`
            (`self.Custom Crouch`))
          (:`B`
            (`self.Custom UnCrouch`))))))
  (:`Completed`
    (goto _label_2 :!via `Reset`)))

(event `EnhancedInput|/Game/Hunters_Field/Data/IA_Jump`
  (params (ActionValue :type Boolean) (ElapsedSeconds :type "Float (double-precision)") (TriggeredSeconds :type "Float (double-precision)") (InputAction :type "InputAction Object Reference" :default "/Game/Hunters_Field/Data/IA_Jump.IA_Jump"))
  ;[0.01938 0.01938 0.01938] Jumping
  (:`Triggered`
    (set `self.bJumping` true)
    (`self.Jump`)
    (`self.Stop`))
  (:`Completed`
    (set `self.bJumping` false)))

(event `EnhancedInput|/Game/Hunters_Field/Data/IA_Sprint`
  (params (ActionValue :type Boolean) (ElapsedSeconds :type "Float (double-precision)") (TriggeredSeconds :type "Float (double-precision)") (InputAction :type "InputAction Object Reference" :default "/Game/Hunters_Field/Data/IA_Sprint.IA_Sprint"))
  (bind _charactermovement (`self.CharacterMovement`))
  ;[0.02029 0.02029 0.02029] Sprinting
  (:`Triggered`
    (set `self.bRunning` true)
    (if (`NavMovementComponent.IsFalling` _charactermovement)
      _
      (elif (`self.bCrouched?`)
        _
        (elif (not (`self.bAiming`))
          (set `CharacterMovementComponent.MaxWalkSpeed` 1000.0 _charactermovement)
          (bind (_direction _fov) (`Timeline|FOV` :!label _label_3)
            (:`Update`
              (set `PlayerCameraManager.DefaultFOV` _fov (`GameplayStatics.GetPlayerCameraManager` 0))))))))
  (:`Completed`
    (set `self.bRunning` false)
    (set `CharacterMovementComponent.MaxWalkSpeed` 500.0 (`self.CharacterMovement`) :!label _label_4)
    (goto _label_3 :!via `Reverse`)))

(event `Stop`
  ;[0.02029 0.02029 0.02029] Sprinting
  (goto _label_4))

(event `EnhancedInput|/Game/Hunters_Field/Data/IA_Aim`
  (params (ActionValue :type Boolean) (ElapsedSeconds :type "Float (double-precision)") (TriggeredSeconds :type "Float (double-precision)") (InputAction :type "InputAction Object Reference" :default "/Game/Hunters_Field/Data/IA_Aim.IA_Aim"))
  (bind _charactermovement (`self.CharacterMovement`))
  ;[0.01938 0.01938 0.01938] Aiming
  (:`Triggered`
    (if (`self.bRunning`)
      (`self.Stop`))
    (set `CharacterMovementComponent.MaxWalkSpeed` 350.0 _charactermovement)
    (set `self.bAiming` true))
  (:`Completed`
    (set `self.bAiming` false)
    (set `CharacterMovementComponent.MaxWalkSpeed` 500.0 _charactermovement)))

(event `self.ReceiveTick`
  (params (DeltaSeconds :type "Float (single-precision)"))
  (bind _camera (`self.Camera`))
  ;[0.0137 0.0137 0.0137] Adding the line trace for procedual gun
  (bind (_outhit _returnvalue) (`KismetSystemLibrary.LineTraceSingle` (`SceneComponent.K2_GetComponentLocation` (`self.Camera`)) (+ (`SceneComponent.K2_GetComponentLocation` _camera) (* (`SceneComponent.GetForwardVector` _camera) (70.0 70.0 70.0))) "TraceTypeQuery1"))
  (set `self.CloseToWall` _returnvalue))

(fn `UserConstructionScript`)