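; Wolf animal Blueprint for a hunting field that roams on spawn and reacts to being damaged.
; Taking damage sets a GetHit flag and applies damage, then either awards points and dies, or clears the flag after a short delay and runs.
; Roaming, damage, death and fleeing logic are called functions not defined here, and construction defers to the parent script.
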(event `self.ReceiveBeginPlay`
  (`self.Rome Around`))

(event `self.ReceiveAnyDamage`
  (params (Damage :type "Float (single-precision)") (DamageType :type "DamageType Object Reference") (InstigatedBy :type "Controller Object Reference") (DamageCauser :type "Actor Object Reference"))
  (set `self.GetHit` true)
  (`self.Damage`)
  (if (`self.IsDead`)
    (`self.Increase Point` 100.0)
    (`self.Die`)
    (else
      (`KismetSystemLibrary.Delay` 0.3)
      (set `self.GetHit` false)
      (`self.Run`))))

(fn `UserConstructionScript`
  (`parent.UserConstructionScript`))