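; BP_Animal is a huntable animal with events for wandering, fleeing, taking damage, awarding points and dying.
; RomeAround walks to a random reachable point, pauses and calls itself again on success, while Run makes one move to a random point at a fixed speed.
; Damage subtracts fixed health and flags death, IncreasePoint adds to the player character's Points, and Die ragdolls the mesh before destroying the actor.
; Nothing in this Blueprint calls Damage, IncreasePoint, Run or Die.
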(event `Rome Around`
  ;[0.01764 0.01764 0.01764] Rome Around
  (set `CharacterMovementComponent.MaxWalkSpeed` (`self.Speed`) (`self.CharacterMovement`))
  (`|AIMoveTo` self (`NavigationSystemV1.K2_GetRandomReachablePointInRadius` (`self.K2_GetActorLocation`) (`self.Radius`) null null) null 150.0
    (:`OnSuccess`
      (set `CharacterMovementComponent.MaxWalkSpeed` 0.0 (`self.CharacterMovement`))
      (`KismetSystemLibrary.Delay` 5.0)
      (`self.Rome Around`))))

(event `Damage`
  ;[0.0185 0.0185 0.0185] Damage
  (set `self.Health` (- (`self.Health`) 50.0))
  (if (<= (`self.Health`) 0.0)
    (set `self.IsDead` true)))

(event `Increase Point`
  (params (Point_Value :type "Float (double-precision)"))
  ;[0.016 0.016 0.016] Increase Point
  (bind _asbp_fps_character (cast `/Game/Hunters_Field/Core/BP_FPS_Character` (`GameplayStatics.GetPlayerCharacter` 0)))
  (set `/Game/Hunters_Field/Core/BP_FPS_Character.Points` (+ Point_Value (`/Game/Hunters_Field/Core/BP_FPS_Character.Points` _asbp_fps_character)) _asbp_fps_character))

(event `Run`
  ;[0.01938 0.01938 0.01938] Run
  (set `CharacterMovementComponent.MaxWalkSpeed` 360.0 (`self.CharacterMovement`))
  (`|AIMoveTo` self (`NavigationSystemV1.K2_GetRandomReachablePointInRadius` (`self.K2_GetActorLocation`) 1000.0 null null) null 150.0
    (:`OnSuccess`
      (set `CharacterMovementComponent.MaxWalkSpeed` 0.0 (`self.CharacterMovement`)))))

(event `Die`
  ;[0.0185 0.0185 0.0185] Die
  (`PrimitiveComponent.SetSimulatePhysics` (`self.Mesh`) true)
  (`KismetSystemLibrary.Delay` 3.0)
  (`self.K2_DestroyActor`))

(fn `UserConstructionScript`)